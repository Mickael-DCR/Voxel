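; Player controller that routes Enhanced Input to BP_PlayerCharacter for movement, aim, firing, zoom and potions, plus keys for inventory and quest log.
; On BeginPlay it creates the inventory and quest log widgets, then initializes stats.
; Inventory and quest component events update character stats, quest counters and UI.
; ResetDungeon respawns the player and resets every enemy spawner.
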(event `self.ReceiveBeginPlay`
  (`EnhancedInputSubsystemInterface.AddMappingContext` (subsystem `EnhancedInputLocalPlayerSubsystem`) "/Game/Developers/Mickael/Inputs/IMC_Default_M.IMC_Default_M" 0 (struct))
  (bind _asbp_player_character (cast `/Game/Blueprints/BP_PlayerCharacter` (`GameplayStatics.GetPlayerPawn` 0)))
  (set `self.Player Character` _asbp_player_character)
  ; Init custom UI then dependencies that rely on it
  (`self.InitUI`)
  (`self.InitDependencies`))

(event `EnhancedInput|/Game/Input/Actions/IA_Look`
  (params (ActionValue :type "Vector2D Structure") (ElapsedSeconds :type "Float (double-precision)") (TriggeredSeconds :type "Float (double-precision)") (InputAction :type "InputAction Object Reference" :default "/Game/Input/Actions/IA_Look.IA_Look"))
  ; Player Character Controls
  (:`Triggered`
    (`/Game/Blueprints/BP_PlayerCharacter.Aim` (`self.Player Character`) ActionValue_X ActionValue_Y)))

(event `self.AC_Inventory.EquipedItemChanged`
  ; Delegates
  (bind _values (`BlueprintMapLibrary.Map_Values` (`/Game/Blueprints/ActorComponents/AC_Inventory.EquipedSlots` (`self.AC_Inventory`))))
  (`/Game/Blueprints/ActorComponents/AC_CharacterStats.UpdateItemValues` (`self.AC_CharacterStats`) _values)
  (`/Game/Blueprints/UI/WBP_Inventory.UpdateStatsDisplay` (`self.UI_Inventory`)))

(event `EnhancedInput|/Game/Developers/Mickael/Inputs/Action/IA_PrimaryFire`
  (params (ActionValue :type Boolean) (ElapsedSeconds :type "Float (double-precision)") (TriggeredSeconds :type "Float (double-precision)") (InputAction :type "InputAction Object Reference" :default "/Game/Developers/Mickael/Inputs/Action/IA_PrimaryFire.IA_PrimaryFire"))
  ; Player Character Controls
  (:`Triggered`
    (`/Game/Blueprints/BP_PlayerCharacter.PrimaryFire` (`self.Player Character`))))

(event `EnhancedInput|/Game/Input/Actions/IA_Move`
  (params (ActionValue :type "Vector2D Structure") (ElapsedSeconds :type "Float (double-precision)") (TriggeredSeconds :type "Float (double-precision)") (InputAction :type "InputAction Object Reference" :default "/Game/Input/Actions/IA_Move.IA_Move"))
  ; Player Character Controls
  (:`Triggered`
    (`/Game/Blueprints/BP_PlayerCharacter.Move` (`self.Player Character`) ActionValue_X ActionValue_Y)))

(event `self.AC_QuestLog.QuestFinished`
  ; Delegates
  (`/Game/Blueprints/UI/WBP_QuestLog.RefreshAllDisplays` (`self.UI_Quests`))
  (`/Game/Blueprints/UI/WBP_Inventory.UpdateStatsDisplay` (`self.UI_Inventory`)))

(event `EnhancedInput|/Game/Developers/Mickael/Inputs/Action/IA_SecondaryFire`
  (params (ActionValue :type Boolean) (ElapsedSeconds :type "Float (double-precision)") (TriggeredSeconds :type "Float (double-precision)") (InputAction :type "InputAction Object Reference" :default "/Game/Developers/Mickael/Inputs/Action/IA_SecondaryFire.IA_SecondaryFire"))
  ; Player Character Controls
  (:`Triggered`
    (`/Game/Blueprints/BP_PlayerCharacter.SecondaryFire` (`self.Player Character`))))

(event `self.AC_Inventory.TrashedItem`
  ; Delegates
  (`/Game/Blueprints/ActorComponents/AC_QuestLog.IncreaseStat` (`self.AC_QuestLog`) (enumliteral `/Game/Blueprints/Data/E_GlobalStats` "NewEnumerator1") 1))

(event `EnhancedInput|/Game/Input/Actions/IA_Jump`
  (params (ActionValue :type Boolean) (ElapsedSeconds :type "Float (double-precision)") (TriggeredSeconds :type "Float (double-precision)") (InputAction :type "InputAction Object Reference" :default "/Game/Input/Actions/IA_Jump.IA_Jump"))
  ; Player Character Controls
  (:`Started`
    (`Character.Jump` (`self.Player Character`))))

(event `Key|C`
  (params (Key :type "Key Structure"))
  ; Interface
  ;; Open Quest Log
  (:`Pressed`
    (`/Game/Blueprints/ActorComponents/AC_QuestLog.ToggleUI` (`self.AC_QuestLog`))))

(event `EnhancedInput|/Game/Developers/Mickael/Inputs/Action/IA_CameraZoom`
  (params (ActionValue :type "Float (double-precision)") (ElapsedSeconds :type "Float (double-precision)") (TriggeredSeconds :type "Float (double-precision)") (InputAction :type "InputAction Object Reference" :default "/Game/Developers/Mickael/Inputs/Action/IA_CameraZoom.IA_CameraZoom"))
  ; Player Character Controls
  (:`Triggered`
    (`/Game/Blueprints/BP_PlayerCharacter.AdjustCameraZoom` (`self.Player Character`) ActionValue)))

(event `EnhancedInput|/Game/Developers/Mickael/Inputs/Action/IA_HealthPotion`
  (params (ActionValue :type Boolean) (ElapsedSeconds :type "Float (double-precision)") (TriggeredSeconds :type "Float (double-precision)") (InputAction :type "InputAction Object Reference" :default "/Game/Developers/Mickael/Inputs/Action/IA_HealthPotion.IA_HealthPotion"))
  ; Player Character Controls
  (:`Started`
    (`/Game/Blueprints/BP_PlayerCharacter.UseHealthPotion` (`self.Player Character`))))

(event `Key|X`
  (params (Key :type "Key Structure"))
  ; Interface
  ;; Delete hovered item
  (:`Pressed`
    (`/Game/Blueprints/ActorComponents/AC_Inventory.DeleteHoveredItem` (`self.AC_Inventory`))))

(event `Key|B`
  (params (Key :type "Key Structure"))
  ; Interface
  ;; Open inventory
  (:`Pressed`
    (`/Game/Blueprints/ActorComponents/AC_Inventory.ToggleUI` (`self.AC_Inventory`))))

(fn `InitDependencies`
  (`/Game/Blueprints/ActorComponents/AC_CharacterStats.InitStats` (`self.AC_CharacterStats`)))

(fn `InitUI`
  (bind _returnvalue (`|CreateWidget` "/Game/Blueprints/UI/WBP_Inventory.WBP_Inventory_C"))
  (bind _output_get (set `self.UI_Inventory` _returnvalue))
  (`/Game/Blueprints/UI/WBP_Inventory.InitBag` _output_get (`/Game/Blueprints/ActorComponents/AC_Inventory.Size` (`self.AC_Inventory`)))
  (bind _returnvalue_2 (`|CreateWidget` "/Game/Blueprints/UI/WBP_QuestLog.WBP_QuestLog_C"))
  (set `self.UI_Quests` _returnvalue_2))

(fn `ResetDungeon`
  (`/Game/Blueprints/BP_PlayerCharacter.Respawn` (`/Game/Blueprints/BPFL_Getters.GetPlayerCharacter`))
  (bind _outactors (`GameplayStatics.GetAllActorsOfClass` "/Game/Blueprints/Enemies/Spawn/BP_EnemySpawner.BP_EnemySpawner_C"))
  (for _array_element _outactors
    (`/Game/Blueprints/Enemies/Spawn/BP_EnemySpawner.ResetSpawns` _array_element)))

(fn `UserConstructionScript`)