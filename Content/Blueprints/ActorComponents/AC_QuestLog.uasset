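; AC_QuestLog is an actor component that tracks quest progress, global stats and the quest log UI.
; On BeginPlay it loads every DT_Quests row into a Quests map as availability and finished flags, unlocking only the first.
; Claiming an eligible quest marks it finished, grants its reward, unlocks its NextQuests and signals completion.
; Stat increases refresh the quest UI, which ToggleUI shows or hides along with the mouse cursor.
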(event `self.ReceiveBeginPlay`
  (`self.InitQuests`))

(fn `ClaimQuest`
  (params (QuestName :type Name))
  (bind _value (`BlueprintMapLibrary.Map_Find` (`self.Quests`) QuestName))
  (bind (_quest _isavailable _isfinished) (break `/Game/Blueprints/Data/F_QuestTracking` _value))
  (if (and (`/Game/Blueprints/FunctionLibraries/BPFL_UtilsQuests.IsClaimable` _quest) _isavailable (not _isfinished))
    (bind _structout (setmembers `/Game/Blueprints/Data/F_QuestTracking` :`StructRef` _value :`IsFinished` true))
    (`BlueprintMapLibrary.Map_Add` (`self.Quests`) (`local.QuestName`) _structout)
    (`/Game/Blueprints/FunctionLibraries/BPFL_UtilsQuests.AcquireReward` _quest)
    (for _array_element (`.NextQuests_11_057FA5244AF4D84C6E153186BEDBDBC1` (break `/Game/Blueprints/Data/F_Quest` _quest))
      (bind (_datatable _rowname) (break `DataTableRowHandle` _array_element))
      (bind _structout_2 (setmembers `/Game/Blueprints/Data/F_QuestTracking` :`StructRef` (`BlueprintMapLibrary.Map_Find` (`self.Quests`) _rowname) :`IsAvailable` true))
      (`BlueprintMapLibrary.Map_Add` (`self.Quests`) _rowname _structout_2))
    (`self.QuestFinished`)
    (else
      (`KismetSystemLibrary.PrintString` "Cannot claim quest" true true (struct :`R` 1.0 :`G` 0.002225 :`A` 1.0)))))

(fn `IncreaseStat`
  (params (Stat :type "/Game/Blueprints/Data/E_GlobalStats Enum (by ref)") (Value :type Integer))
  (`BlueprintMapLibrary.Map_Add` (`self.GlobalStats`) (`local.Stat`) (+ (`BlueprintMapLibrary.Map_Find` (`self.GlobalStats`) (`local.Stat`)) (`local.Value`)))
  (`/Game/Blueprints/UI/WBP_QuestLog.RefreshAllDisplays` (`/Game/Blueprints/BP_PlayerController.UI_Quests` (`/Game/Blueprints/BPFL_Getters.GetPlayerController`))))

(fn `InitQuests`
  (bind _quests (`self.Quests`))
  (bind (_key _value) (`BlueprintMapLibrary.Map_GetKeyValueByIndex` _quests))
  (bind _outrownames (`DataTableFunctionLibrary.GetDataTableRowNames` "/Game/Blueprints/Data/Quests/DT_Quests.DT_Quests"))
  (for _array_element _outrownames
    (bind _returnvalue (`|GetDataTableRow` "/Game/Blueprints/Data/Quests/DT_Quests.DT_Quests" _array_element)
      (:`then`
        (`BlueprintMapLibrary.Map_Add` (`self.Quests`) _array_element (make `/Game/Blueprints/Data/F_QuestTracking` _returnvalue)))))
  ; Init first quest
  (bind _structout (setmembers `/Game/Blueprints/Data/F_QuestTracking` :`StructRef` _value :`IsAvailable` true))
  (`BlueprintMapLibrary.Map_Add` _quests _key _structout))

(fn `ToggleUI`
  (bind _asbp_player_controller (`/Game/Blueprints/BPFL_Getters.GetPlayerController`))
  (bind _ui_quests (`/Game/Blueprints/BP_PlayerController.UI_Quests` _asbp_player_controller))
  (bind _output_get (set `self.IsDisplayed` (not (`self.IsDisplayed`))))
  (if _output_get
    (`UserWidget.AddToViewport` _ui_quests 0)
    (set `PlayerController.bShowMouseCursor` true _asbp_player_controller)
    (`/Game/Blueprints/UI/WBP_QuestLog.RefreshAllDisplays` _ui_quests)
    (else
      (`Widget.RemoveFromParent` _ui_quests)
      (set `PlayerController.bShowMouseCursor` false _asbp_player_controller))))