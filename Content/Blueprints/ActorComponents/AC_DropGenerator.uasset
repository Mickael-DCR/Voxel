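; Actor component that rolls loot from drop rules and puts the items straight into the player's inventory bag.
; DrawForRules makes one draw per rule from its DataTable, then adds valid results and prints their names.
; Both draws use cumulative probability: weighted rolls against the table's total, while stochastic rolls against 100, so it can yield nothing.
; The winning row's item handle resolves to the item data.
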(fn `DrawForRules`
  (params (DropRules :type "Array of /Game/Blueprints/Data/F_DropRule Structure"))
  (locals (LootToSpawn :type "Array of /Game/Blueprints/Data/F_Item Structure"))
  (for _array_element DropRules
    (bind (_droptable _isweighted) (break `/Game/Blueprints/Data/F_DropRule` _array_element))
    (if _isweighted
      (bind _item (`self.DrawWeighted` _droptable))
      (`KismetArrayLibrary.Array_Add` (`local.LootToSpawn`) _item)
      (else
        (bind _item_2 (`self.DrawStochastic` _droptable))
        (`KismetArrayLibrary.Array_Add` (`local.LootToSpawn`) _item_2))))
  (for _array_element_2 (`local.LootToSpawn`)
    (if (`/Game/Blueprints/FunctionLibraries/BPFL_UtilsItems.IsValid` _array_element_2)
      (`/Game/Blueprints/ActorComponents/AC_Inventory.AddItemToBag` (`/Game/Blueprints/BP_PlayerController.AC_Inventory` (`/Game/Blueprints/BPFL_Getters.GetPlayerController`)) _array_element_2)
      (`KismetSystemLibrary.PrintString` (`KismetStringLibrary.Concat_StrStr` "Loot : " (`.Name_5_E0B6498D42D2C3F2CB9DAAAAB379317A` (break `/Game/Blueprints/Data/F_Item` _array_element_2)))))))

(fn `DrawStochastic`
  (params (DropTable :type "DataTable Object Reference"))
  (returns (Item :type "/Game/Blueprints/Data/F_Item Structure"))
  (locals (Cumulated :type "Float (double-precision)") (Seed :type "Float (double-precision)" :default 0.0))
  (set `local.Cumulated` 0.0)
  (set `local.Seed` (`KismetMathLibrary.RandomFloatInRange` 0.0 100.0))
  (bind _outrownames (`DataTableFunctionLibrary.GetDataTableRowNames` DropTable))
  (for _array_element _outrownames
    (bind _returnvalue (`|GetDataTableRow` (`local.DropTable`) _array_element)
      (:`then`
        (bind (_item _probability) (break `/Game/Blueprints/Data/F_Drop` _returnvalue))
        (if (>= (+ _probability (`local.Cumulated`)) (`local.Seed`))
          (bind (_datatable _rowname) (break `DataTableRowHandle` _item))
          (bind _returnvalue_2 (`|GetDataTableRow` _datatable _rowname)
            (:`then`
              (return _returnvalue_2)))
          (else
            (set `local.Cumulated` (+ _probability (`local.Cumulated`))))))))
  (return))

(fn `DrawWeighted`
  (params (DropTable :type "DataTable Object Reference"))
  (returns (Item :type "/Game/Blueprints/Data/F_Item Structure"))
  (locals (Total :type "Float (double-precision)") (Cumulated :type "Float (double-precision)") (Seed :type "Float (double-precision)"))
  (set `local.Total` 0.0)
  (`|ExecutionSequence`
    (:`then_0`
      ; Init chances
      (bind _outrownames (`DataTableFunctionLibrary.GetDataTableRowNames` DropTable))
      (for _array_element _outrownames
        (bind _returnvalue (`|GetDataTableRow` (`local.DropTable`) _array_element)
          (:`then`
            (set `local.Total` (+ (`.Probability_7_6BC579A94DF55A42EBCEA5B7F6AC1A12` (break `/Game/Blueprints/Data/F_Drop` _returnvalue)) (`local.Total`))))))
      (set `local.Seed` (`KismetMathLibrary.RandomFloatInRange` 0.0 (`local.Total`))))
    (:`then_1`
      (set `local.Cumulated` 0.0)
      (bind _outrownames_2 (`DataTableFunctionLibrary.GetDataTableRowNames` DropTable))
      (for _array_element_2 _outrownames_2
        (bind _returnvalue_2 (`|GetDataTableRow` (`local.DropTable`) _array_element_2)
          (:`then`
            (bind (_item _probability) (break `/Game/Blueprints/Data/F_Drop` _returnvalue_2))
            (if (>= (+ _probability (`local.Cumulated`)) (`local.Seed`))
              (bind (_datatable _rowname) (break `DataTableRowHandle` _item))
              (bind _returnvalue_3 (`|GetDataTableRow` _datatable _rowname)
                (:`then`
                  (return _returnvalue_3)))
              (else
                (set `local.Cumulated` (+ _probability (`local.Cumulated`))))))))
      (return))))