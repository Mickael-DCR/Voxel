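; Actor component that manages a character's inventory: a fixed-size bag array plus an equipment map keyed by item slot enum.
; Adding, equipping (swapping with the bag), unequipping and deleting route through two setters that update the player controller's UIInventory widget, with equipment changes also firing a change notification.
; It also toggles the inventory UI and cursor, tracks the hovered slot for trashing items, and prints contents for debugging.
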(event `self.ReceiveBeginPlay`
  (`self.InitSlots`))

(fn `AddItemToBag`
  (params (Item :type "/Game/Blueprints/Data/F_Item Structure"))
  (returns (Added :type Boolean))
  (locals (FoundIndex :type Integer :default 0))
  (if (not (`self.CheckIsFull`))
    (bind _output_get (set `local.FoundIndex` (`self.FindFirstEmptyBagIndex`)))
    (`self.SetItemInBagIndex` _output_get (`local.Item`))
    (return true)
    (else
      (`KismetSystemLibrary.PrintString` "Error: Inventory is full" true true (struct :`R` 1.0 :`A` 1.0))
      (return false))))

(fn `CheckIsFull`
  (returns (IsFull :type Boolean))
  (locals (counter :type Integer))
  (for _array_element (`self.BagItems`)
    (if (`/Game/Blueprints/FunctionLibraries/BPFL_UtilsItems.IsValid` _array_element)
      (`/Engine/EditorBlueprintResources/StandardMacros.IncrementInt` (`local.counter`))))
  (return (>= (`local.counter`) (`self.Size`))))

(fn `DeleteHoveredItem`
  (bind _hoveredslot (`self.HoveredSlot`))
  (`/Engine/EditorBlueprintResources/StandardMacros.IsValid` _hoveredslot
    (:`Is Valid`
      (if (`/Game/Blueprints/FunctionLibraries/BPFL_UtilsItems.IsValid` (`/Game/Blueprints/UI/WBP_ItemSlot.Item` _hoveredslot))
        (`/Game/Blueprints/UI/WBP_ItemSlot.DeleteItem` _hoveredslot)
        (`self.TrashedItem`)
        (else
          (`KismetSystemLibrary.PrintString` "No item to delete" true true (struct :`R` 1.0 :`G` 0.037559 :`A` 1.0) :!label _label))))
    (:`Is Not Valid`
      (goto _label))))

(fn `DeleteItemFromBag`
  (params (Index :type Integer))
  (`self.SetItemInBagIndex` Index))

(fn `DeleteItemFromEquipedSlot`
  (params (Index :type "/Game/Blueprints/Data/E_ItemSlot Enum" :default "NewEnumerator0"))
  (`self.SetItemInEquipedSlot` Index))

(fn `EquipItemFromBag`
  (params (index :type Integer))
  (locals (ItemToBag :type "/Game/Blueprints/Data/F_Item Structure") (ItemToEquip :type "/Game/Blueprints/Data/F_Item Structure"))
  (bind _output (`|GetArrayItem` (`self.BagItems`) index))
  (if (`/Game/Blueprints/FunctionLibraries/BPFL_UtilsItems.IsValid` _output)
    (bind _output_get (set `local.ItemToEquip` _output))
    (set `local.ItemToBag` (`BlueprintMapLibrary.Map_Find` (`self.EquipedSlots`) (`.Slot_15_7DF818094A48FDB2BF11EF929B5E6AF2` (break `/Game/Blueprints/Data/F_Item` _output_get))))
    (`self.SetItemInBagIndex` (`local.index`) (`local.ItemToBag`))
    (`self.SetItemInEquipedSlot` (`.Slot_15_7DF818094A48FDB2BF11EF929B5E6AF2` (break `/Game/Blueprints/Data/F_Item` _output_get)) (`local.ItemToEquip`))
    (else
      (`KismetSystemLibrary.PrintString` "Error: cannot equip" true true (struct :`R` 1.0 :`A` 1.0)))))

(fn `FindFirstEmptyBagIndex`
  (returns (Index :type Integer))
  (for (_array_element _array_index) (`self.BagItems`)
    (if (not (`/Game/Blueprints/FunctionLibraries/BPFL_UtilsItems.IsValid` _array_element))
      (return _array_index)))
  (return -1))

(fn `InitSlots`
  (`KismetArrayLibrary.Array_Resize` (`self.BagItems`) (`self.Size`))
  (bind _enumvalue (foreach `/Game/Blueprints/Data/E_ItemSlot` false)
    (:`LoopBody`
      (`BlueprintMapLibrary.Map_Add` (`self.EquipedSlots`) _enumvalue))))

(fn `MouseEnterSlot`
  (params (ItemSlot :type "/Game/Blueprints/UI/WBP_ItemSlot Object Reference"))
  (set `self.HoveredSlot` ItemSlot))

(fn `MouseLeaveSlot`
  (set `self.HoveredSlot` null))

(fn `PrintContent`
  (bind (_keypin _valuepin) (`|MapForEach` (`self.EquipedSlots`))
    (:`then`
      (if (`/Game/Blueprints/FunctionLibraries/BPFL_UtilsItems.IsValid` _valuepin)
        (`KismetSystemLibrary.PrintString` (`KismetStringLibrary.Concat_StrStr` (`|GetEnumeratorNameAsString` _keypin) ": " (`.Name_5_E0B6498D42D2C3F2CB9DAAAAB379317A` (break `/Game/Blueprints/Data/F_Item` _valuepin))) true true (struct :`G` 0.072392 :`B` 1.0 :`A` 1.0))
        (else
          (`KismetSystemLibrary.PrintString` (`KismetStringLibrary.Concat_StrStr` (`|GetEnumeratorNameAsString` _keypin) ": " "Empty") true true (struct :`G` 0.072392 :`B` 1.0 :`A` 1.0)))))
    (:`CompletedPin`
      (for (_array_element _array_index) (`self.BagItems`)
        (if (`/Game/Blueprints/FunctionLibraries/BPFL_UtilsItems.IsValid` _array_element)
          (`KismetSystemLibrary.PrintString` (`KismetStringLibrary.Concat_StrStr` "(" (`KismetStringLibrary.Conv_IntToString` _array_index) "): " (`.Name_5_E0B6498D42D2C3F2CB9DAAAAB379317A` (break `/Game/Blueprints/Data/F_Item` _array_element))) true true (struct :`G` 1.0 :`B` 0.499469 :`A` 1.0)))))))

(fn `SetItemInBagIndex`
  (params (Index :type Integer) (Item :type "/Game/Blueprints/Data/F_Item Structure (by ref)"))
  (`KismetArrayLibrary.Array_Set` (`self.BagItems`) Index Item)
  (`/Game/Blueprints/UI/WBP_Inventory.ChangeBagItem` (`/Game/Blueprints/BP_PlayerController.UI_Inventory` (`/Game/Blueprints/BPFL_Getters.GetPlayerController`)) (`local.Index`) (`local.Item`)))

(fn `SetItemInEquipedSlot`
  (params (ItemSlot :type "/Game/Blueprints/Data/E_ItemSlot Enum" :default "NewEnumerator0") (Item :type "/Game/Blueprints/Data/F_Item Structure"))
  (`BlueprintMapLibrary.Map_Add` (`self.EquipedSlots`) (`local.ItemSlot`) (`local.Item`))
  (`/Game/Blueprints/UI/WBP_Inventory.ChangeEquipedItem` (`/Game/Blueprints/BP_PlayerController.UI_Inventory` (`/Game/Blueprints/BPFL_Getters.GetPlayerController`)) (`local.ItemSlot`) (`local.Item`))
  (`self.EquipedItemChanged`))

(fn `ToggleUI`
  (bind _asbp_player_controller (`/Game/Blueprints/BPFL_Getters.GetPlayerController`))
  (bind _ui_inventory (`/Game/Blueprints/BP_PlayerController.UI_Inventory` _asbp_player_controller))
  (bind _output_get (set `self.IsDisplayed` (not (`self.IsDisplayed`))))
  (if _output_get
    (`UserWidget.AddToViewport` _ui_inventory 0)
    (set `PlayerController.bShowMouseCursor` true _asbp_player_controller)
    (else
      (`Widget.RemoveFromParent` _ui_inventory)
      (set `PlayerController.bShowMouseCursor` false _asbp_player_controller))))

(fn `UnequipItemFromSlot`
  (params (ItemSlot :type "/Game/Blueprints/Data/E_ItemSlot Enum" :default "NewEnumerator0"))
  (locals (ItemToBag :type "Object Object Reference"))
  (bind _added (`self.AddItemToBag` (`BlueprintMapLibrary.Map_Find` (`self.EquipedSlots`) (`local.ItemSlot`))))
  (if _added
    (`self.SetItemInEquipedSlot` (`local.ItemSlot`))))