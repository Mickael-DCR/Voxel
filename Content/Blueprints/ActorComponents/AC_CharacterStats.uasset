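; Actor component that holds the player's attribute stats, each split into base, quest bonus and item bonus values, with total and detail lookups.
; InitStats builds the stat map from base values for every attribute and refreshes the inventory UI.
; Quest rewards add to the quest bonus, while equipment updates re-sum every equipped item's affixes into the item bonus.
; Both updates notify the player character of max health changes.
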(fn `AddStatQuestValue`
  (params (PlayerAttribute :type "/Game/Blueprints/Data/E_PlayerAttribute Enum (by ref)") (Value :type "Float (double-precision)"))
  (locals (PreviousMaxHealth :type "Float (double-precision)" :default 0.0))
  (bind _asbp_player_character (`/Game/Blueprints/BPFL_Getters.GetPlayerCharacter`))
  (bind _value (`BlueprintMapLibrary.Map_Find` (`self.Stats`) PlayerAttribute))
  (set `local.PreviousMaxHealth` (`/Game/Blueprints/BP_PlayerCharacter.GetMaxHealth` (`/Game/Blueprints/BPFL_Getters.GetPlayerCharacter`)))
  (bind _structout (setmembers `/Game/Blueprints/Data/F_CharacterStat` :`StructRef` _value :`QuestsBonus` (+ (`.QuestsBonus_10_9C75E3E24C163D270F05BBA5A520A572` (break `/Game/Blueprints/Data/F_CharacterStat` _value)) Value)))
  (`BlueprintMapLibrary.Map_Add` (`self.Stats`) (`local.PlayerAttribute`) _structout)
  (`/Game/Blueprints/BP_PlayerCharacter.ChangeMaxHealth` _asbp_player_character (`local.PreviousMaxHealth`) (`/Game/Blueprints/BP_PlayerCharacter.GetMaxHealth` _asbp_player_character)))

(fn `GetStatDetail`
  (params (PlayerAttribute :type "/Game/Blueprints/Data/E_PlayerAttribute Enum (by ref)"))
  (returns (Result :type Text))
  (return (`/Game/Blueprints/FunctionLibraries/BPFL_UtilsStats.GetDetail` (`BlueprintMapLibrary.Map_Find` (`self.Stats`) PlayerAttribute))))

(fn `GetStatValue`
  (params (PlayerAttribute :type "/Game/Blueprints/Data/E_PlayerAttribute Enum (by ref)"))
  (returns (Total :type "Float (double-precision)"))
  (return (`/Game/Blueprints/FunctionLibraries/BPFL_UtilsStats.GetTotal` (`BlueprintMapLibrary.Map_Find` (`self.Stats`) PlayerAttribute))))

(fn `InitStats`
  (bind _ui_inventory (`/Game/Blueprints/BP_PlayerController.UI_Inventory` (`/Game/Blueprints/BPFL_Getters.GetPlayerController`)))
  (bind _enumvalue (foreach `/Game/Blueprints/Data/E_PlayerAttribute` false)
    (:`LoopBody`
      (`BlueprintMapLibrary.Map_Add` (`self.Stats`) _enumvalue (make `/Game/Blueprints/Data/F_CharacterStat` (`BlueprintMapLibrary.Map_Find` (`self.BaseStats`) _enumvalue))))
    (:`then`
      (`/Game/Blueprints/UI/WBP_Inventory.InitStats` _ui_inventory)
      (`/Game/Blueprints/UI/WBP_Inventory.UpdateStatsDisplay` _ui_inventory))))

(fn `UpdateItemValues`
  (params (EquipedItems :type "Array of /Game/Blueprints/Data/F_Item Structure"))
  (locals (TotalValues :type "Map of /Game/Blueprints/Data/E_PlayerAttribute Enum to Float (double-precision)") (PreviousMaxHealth :type "Float (double-precision)"))
  (bind _asbp_player_character (`/Game/Blueprints/BPFL_Getters.GetPlayerCharacter`))
  ; Init totals
  (bind _enumvalue (foreach `/Game/Blueprints/Data/E_PlayerAttribute` false)
    (:`LoopBody`
      (`BlueprintMapLibrary.Map_Add` (`local.TotalValues`) _enumvalue)
      (set `local.PreviousMaxHealth` (`/Game/Blueprints/BP_PlayerCharacter.GetMaxHealth` (`/Game/Blueprints/BPFL_Getters.GetPlayerCharacter`))))
    (:`then`
      ; Loop through every item equipped
      (for _array_element (`local.EquipedItems`)
        ;; Loop through every affix
        (for _array_element_2 (`.Affixes_9_CB908F6F4D7FFC82C3C697B15E4705CD` (break `/Game/Blueprints/Data/F_Item` _array_element))
          (bind (_attribute _value) (break `/Game/Blueprints/Data/F_ItemAffix` _array_element_2))
          (`BlueprintMapLibrary.Map_Add` (`local.TotalValues`) _attribute (+ (`BlueprintMapLibrary.Map_Find` (`local.TotalValues`) _attribute) _value))))
      ; Write total on stats
      (bind (_keypin _valuepin) (`|MapForEach` (`self.Stats`))
        (:`then`
          (bind _structout (setmembers `/Game/Blueprints/Data/F_CharacterStat` :`StructRef` _valuepin :`ItemsBonus` (`BlueprintMapLibrary.Map_Find` (`local.TotalValues`) _keypin)))
          (`BlueprintMapLibrary.Map_Add` (`self.Stats`) _keypin _structout))
        (:`CompletedPin`
          ; Update MaxHealth
          (`/Game/Blueprints/BP_PlayerCharacter.ChangeMaxHealth` _asbp_player_character (`local.PreviousMaxHealth`) (`/Game/Blueprints/BP_PlayerCharacter.GetMaxHealth` _asbp_player_character)))))))