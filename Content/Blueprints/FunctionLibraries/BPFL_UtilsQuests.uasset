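; Function library of quest helpers that formats quest descriptions, checks whether a quest can be claimed and grants its reward.
; Progress comes from the GlobalStats map in the player controller's quest log component, looked up by the quest's stat and compared to its goal.
; Rewards switch on type: attack, defense and health add quest values to the controller's character stats component, while potion charge and percentage healing bonuses go to the player character.
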(fn `AcquireReward`
  (params (Quest :type "/Game/Blueprints/Data/F_Quest Structure"))
  (bind ((`RewardType_22_49A365A64CF5441EF6ED4CACC124479E` _rewardtype) (`RewardQty_23_AB5543BA492BDFA284E4389B964A07C1` _rewardqty)) (break `/Game/Blueprints/Data/F_Quest` Quest))
  (bind _ac_characterstats (`/Game/Blueprints/BP_PlayerController.AC_CharacterStats` (`/Game/Blueprints/BPFL_Getters.GetPlayerController` null)))
  (switch `/Game/Blueprints/Data/E_QuestRewards` _rewardtype
    (:`NewEnumerator0`
      (`/Game/Blueprints/ActorComponents/AC_CharacterStats.AddStatQuestValue` _ac_characterstats (enumliteral `/Game/Blueprints/Data/E_PlayerAttribute` "NewEnumerator2") _rewardqty))
    (:`NewEnumerator1`
      (`/Game/Blueprints/ActorComponents/AC_CharacterStats.AddStatQuestValue` _ac_characterstats (enumliteral `/Game/Blueprints/Data/E_PlayerAttribute` "NewEnumerator1") _rewardqty))
    (:`NewEnumerator2`
      (`/Game/Blueprints/ActorComponents/AC_CharacterStats.AddStatQuestValue` _ac_characterstats (enumliteral `/Game/Blueprints/Data/E_PlayerAttribute` "NewEnumerator0") _rewardqty))
    (:`NewEnumerator3`
      (`/Game/Blueprints/BP_PlayerCharacter.AddPotionCharge` (`/Game/Blueprints/BPFL_Getters.GetPlayerCharacter` null) _rewardqty))
    (:`NewEnumerator4`
      (`/Game/Blueprints/BP_PlayerCharacter.AddPotionHeal` (`/Game/Blueprints/BPFL_Getters.GetPlayerCharacter` null) (/ _rewardqty 100.0)))))

(fn `GetDescription`
  (params (Quest :type "/Game/Blueprints/Data/F_Quest Structure"))
  (returns (Result :type Text))
  (bind ((`Stat_7_0E205E574F47E2EF50AFB890FD8579CE` _stat) (`Goal_9_E33CD95F4818701D2A62D98A8EEE2E58` _goal) (`RewardType_22_49A365A64CF5441EF6ED4CACC124479E` _rewardtype) (`RewardQty_23_AB5543BA492BDFA284E4389B964A07C1` _rewardqty)) (break `/Game/Blueprints/Data/F_Quest` Quest))
  (return (`|FormatText` "{stat} : {progress} / {goal} \nReward : + {qty} {type}" (`|GetEnumeratorNameAsString` _stat) (`BlueprintMapLibrary.Map_Find` (`/Game/Blueprints/ActorComponents/AC_QuestLog.GlobalStats` (`/Game/Blueprints/BP_PlayerController.AC_QuestLog` (`/Game/Blueprints/BPFL_Getters.GetPlayerController` null))) _stat) _goal _rewardqty (`|GetEnumeratorNameAsString` _rewardtype))))

(fn `IsClaimable`
  (params (Quest :type "/Game/Blueprints/Data/F_Quest Structure"))
  (returns (ReturnValue :type Boolean))
  (bind (_stat _goal) (break `/Game/Blueprints/Data/F_Quest` Quest))
  (return (>= (`BlueprintMapLibrary.Map_Find` (`/Game/Blueprints/ActorComponents/AC_QuestLog.GlobalStats` (`/Game/Blueprints/BP_PlayerController.AC_QuestLog` (`/Game/Blueprints/BPFL_Getters.GetPlayerController` null))) _stat) _goal)))