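; Blueprint function library of helpers for item structs, covering a validity check and display text.
; IsValid treats any item with a non-empty Name as valid.
; GetDescription concatenates each affix's attribute and value into one string, then formats it with name, level, rarity and slot, plus hard-coded equip and delete control hints.
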(fn `GetDescription`
  (params (Item :type "/Game/Blueprints/Data/F_Item Structure"))
  (returns (Result :type Text))
  (locals (AffixString :type String))
  (bind (_level _name _affixes _slot _rarity) (break `/Game/Blueprints/Data/F_Item` Item))
  (for _array_element _affixes
    (bind (_attribute _value) (break `/Game/Blueprints/Data/F_ItemAffix` _array_element))
    (set `local.AffixString` (`KismetStringLibrary.Concat_StrStr` (`local.AffixString`) (`KismetTextLibrary.Conv_TextToString` (`|FormatText` " \n{stat} +{value}" (`|GetEnumeratorNameAsString` _attribute) _value)))))
  (return (`|FormatText` "{name} (level {level}) \n{rarity} {slot}{affixes} \nRMB - Equip \nX - Delete" _name _level (`|GetEnumeratorNameAsString` _rarity) (`|GetEnumeratorNameAsString` _slot) (`local.AffixString`))))

(fn `IsValid`
  (params (Item :type "/Game/Blueprints/Data/F_Item Structure"))
  (returns (IsValid :type Boolean))
  (return (`KismetStringLibrary.NotEqual_StrStr` Item_Name_5_E0B6498D42D2C3F2CB9DAAAAB379317A)))