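; BP_EnemySpawner spawns enemies at a set of spawn point actors when play begins.
; Its spawner type either places the first enemy type at every point or pairs each type with the point at the same index.
; Spawned actors are tracked in an array, which KillAll uses to destroy them and ResetSpawns uses to clear and respawn the whole group.
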(event `self.ReceiveBeginPlay`
  (`self.SpawnEnemies`))

(fn `KillAll`
  (if (> (`KismetArrayLibrary.Array_Length` (`self.EnemiesSpawned`)) 0)
    (for _array_element (`self.EnemiesSpawned`)
      (`/Engine/EditorBlueprintResources/StandardMacros.IsValid` _array_element
        (:`Is Valid`
          (`self.K2_DestroyActor` _array_element))))
    (`KismetArrayLibrary.Array_Clear` (`self.EnemiesSpawned`))))

(fn `ResetSpawns`
  (`self.KillAll`)
  (`self.SpawnEnemies`))

(fn `SpawnEnemies`
  (switch `/Game/Blueprints/Enemies/Spawn/E_SpawnerType` (`self.SpawnerType`)
    (:`NewEnumerator0`
      ; Spawns the same type to all spawn points
      (for _array_element (`self.Spawns`)
        (bind _returnvalue (`|SpawnActorFromClass` (`|ConvertAsset` (`|GetArrayItem` (`self.EnemyTypes`))) (`self.GetTransform` _array_element) "Undefined" "MultiplyWithRoot" null null))
        (`KismetArrayLibrary.Array_Add` (`self.EnemiesSpawned`) _returnvalue)))
    (:`NewEnumerator1`
      ; Spawn each type to the same index location
      (for (_array_element_2 _array_index) (`self.EnemyTypes`)
        (bind _returnvalue_2 (`|SpawnActorFromClass` (`|ConvertAsset` _array_element_2) (`self.GetTransform` (`|GetArrayItem` (`self.Spawns`) _array_index)) "Undefined" "MultiplyWithRoot" null null))
        (`KismetArrayLibrary.Array_Add` (`self.EnemiesSpawned`) _returnvalue_2)))))

(fn `UserConstructionScript`)