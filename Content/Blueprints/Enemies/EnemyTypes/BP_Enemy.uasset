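; Base enemy character that fights the player, drops loot and advances quest progress on death.
; BeginPlay loads stats and drop rules from its Monster data table row; a health bar widget rotates to face the camera each tick.
; AttackPlayer damages the given target if a sphere trace around the enemy finds it, then plays a montage.
; Incoming damage is reduced by Defense; at zero health it triggers the player controller's drop and quest-log components, then destroys itself.
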(event `self.ReceiveBeginPlay`
  (`self.SetUpStats`)
  (bind _aswbp_enemy_widget (cast `/Game/Blueprints/UI/WBP_EnemyWidget` (`WidgetComponent.GetWidget` (`self.HealthBar`))))
  (set `self.HealthBarWidget` _aswbp_enemy_widget))

(event `self.ReceiveTick`
  (params (DeltaSeconds :type "Float (single-precision)"))
  ; Rotates the widget to face the camera
  (`SceneComponent.K2_SetWorldRotation` (`self.HealthBar`) (`KismetMathLibrary.FindLookAtRotation` (`SceneComponent.K2_GetComponentLocation` (`self.HealthBar`)) (`SceneComponent.K2_GetComponentLocation` (`PlayerCameraManager.TransformComponent` (`GameplayStatics.GetPlayerCameraManager` 0)))) false false))

(event `self.ReceiveAnyDamage`
  (params (Damage :type "Float (single-precision)") (DamageType :type "DamageType Object Reference") (InstigatedBy :type "Controller Object Reference") (DamageCauser :type "Actor Object Reference"))
  (bind _output_get (set `self.Health` (- (`self.Health`) (- Damage (`self.Defense`)))))
  (`/Game/Blueprints/UI/WBP_EnemyWidget.UpdateHealth` (`self.HealthBarWidget`) (/ _output_get (`self.MaxHealth`)))
  (if (<= _output_get 0.0)
    (`self.Die`)))

(event `/Game/Blueprints/Enemies/Behaviour/BPI_Enemy.AttackPlayer`
  (params (Target :type "Actor Object Reference"))
  (bind _returnvalue (`self.K2_GetActorLocation`))
  (bind (_outhits _returnvalue_2) (`KismetSystemLibrary.SphereTraceMultiForObjects` _returnvalue _returnvalue 200.0 (`|MakeArray` "ObjectTypeQuery3" :!type "EObjectTypeQuery Enum")))
  (if _returnvalue_2
    (for _array_element _outhits
      (bind (_bblockinghit _binitialoverlap _time _distance _location _impactpoint _normal _impactnormal _physmat _hitactor) (`GameplayStatics.BreakHitResult` _array_element))
      (if (== Target _hitactor)
        (`GameplayStatics.ApplyDamage` _hitactor (`self.Attack`))
        (`|PlayMontage` (`self.Mesh`) "/Game/Characters/Mannequins/Anims/Unarmed/Attack/MM_Attack_01_Montage.MM_Attack_01_Montage"
          (:`then`
            (break)))))))

(fn `Die`
  ; Loot drop logic
  (`/Game/Blueprints/ActorComponents/AC_DropGenerator.DrawForRules` (`/Game/Blueprints/BP_PlayerController.AC_DropGenerator` (`/Game/Blueprints/BPFL_Getters.GetPlayerController`)) (`self.Drop Rules`))
  ; Quest progress
  (`/Game/Blueprints/ActorComponents/AC_QuestLog.IncreaseStat` (`/Game/Blueprints/BP_PlayerController.AC_QuestLog` (`/Game/Blueprints/BPFL_Getters.GetPlayerController`)) (enumliteral `/Game/Blueprints/Data/E_GlobalStats` "NewEnumerator0") 1)
  (`self.K2_DestroyActor`))

(fn `SetUpStats`
  (bind (_monster_datatable _monster_rowname) (break `DataTableRowHandle` (`self.Monster`)))
  (bind _returnvalue (`|GetDataTableRow` _monster_datatable _monster_rowname)
    (:`then`
      (bind (_name _health _attack _speed _droprules) (break `/Game/Blueprints/Data/F_Monster` _returnvalue))
      (bind _output_get (set `self.MaxHealth` _health))
      (set `self.Health` _output_get)
      (set `self.Attack` _attack)
      (set `self.Speed` (* _speed 80.0))
      (set `self.Drop Rules` _droprules)
      (set `CharacterMovementComponent.MaxWalkSpeed` (`self.Speed`) (`self.CharacterMovement`)))))

(fn `UserConstructionScript`)